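; TestBRSBP is a test Creature-animated actor that the player moves left and right with keyboard input.
; The MoveLeftRight axis always pushes it along local -X by the absolute input, without sweep or delta-time scaling, so rotation decides direction.
; A and D set opposite facings, flipping Y scale to mirror the mesh, and toggle the IsMove condition on the CreatureMesh state machine.
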(event EventBeginPlay)

(event EventActorBeginOverlap
  (params (OtherActor :type Actor%20Object%20Reference)))

(event EventTick
  (params (DeltaSeconds :type Float%20%28single-precision%29)))

(event Input|AxisEvents|InputAxisMoveLeftRight
  (params (AxisValue :type Float%20%28single-precision%29))
  (Transformation|AddActorLocalOffset (* "-1.000000,0.000000, 0" (Math|Float|Absolute(Float) AxisValue)) false false))

(event Input|KeyboardEvents|A
  (params (Key :type Key%20Structure :default "AnyKey"))
  (bind _returnvalue (Transformation|GetActorScale3D))
  (bind (_x _y _z) (Math|Vector|BreakVector _returnvalue))
  (:Pressed
    (Transformation|SetActorRotation "0,0.000000, 0")
    (Transformation|SetActorScale3D (Math|Vector|MakeVector _x (Math|Float|Absolute(Float) _y) _z))
    (Class|CreatureAnimStateMachine|SetCondition (Variables|/Script/CreaturePlugin.CreatureMeshComponent|GetStateMachineAsset (Variables|Default|GetCreatureMesh)) "IsMove" true))
  (:Released
    (Class|CreatureAnimStateMachine|SetCondition (Variables|/Script/CreaturePlugin.CreatureMeshComponent|GetStateMachineAsset (Variables|Default|GetCreatureMesh)) "IsMove" false)))

(event Input|KeyboardEvents|D
  (params (Key :type Key%20Structure :default "AnyKey"))
  (bind _returnvalue (Transformation|GetActorScale3D))
  (bind (_x _y _z) (Math|Vector|BreakVector _returnvalue))
  (:Pressed
    (Transformation|SetActorRotation "0,180.000000, 0")
    (Transformation|SetActorScale3D (Math|Vector|MakeVector _x (* (Math|Float|Absolute(Float) _y) -1.0) _z))
    (Class|CreatureAnimStateMachine|SetCondition (Variables|/Script/CreaturePlugin.CreatureMeshComponent|GetStateMachineAsset (Variables|Default|GetCreatureMesh)) "IsMove" true))
  (:Released
    (Class|CreatureAnimStateMachine|SetCondition (Variables|/Script/CreaturePlugin.CreatureMeshComponent|GetStateMachineAsset (Variables|Default|GetCreatureMesh)) "IsMove" false)))

(fn ConstructionScript)